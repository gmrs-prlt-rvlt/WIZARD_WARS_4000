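; Water killzone actor that drains health from characters submerged below the height of its static mesh.
; Every Tick it gathers all ThirdPersonCharacter actors and calls DamageHealth with a small fixed amount on any sitting more than 150 units below the mesh.
; The test compares only Z, with no overlap or horizontal bounds, so it applies level-wide.
; Damage is per frame, unscaled by delta time.
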(event EventBeginPlay)

(event Collision|EventActorBeginOverlap
  (params (OtherActor :type Actor%20Object%20Reference)))

(event EventTick
  (params (DeltaSeconds :type Float%20%28single-precision%29))
  (bind _outactors (Actor|GetAllActorsOfClass "/Game/ThirdPersonBP/Blueprints/ThirdPersonCharacter.ThirdPersonCharacter_C"))
  (for _array_element _outactors
    (if (< (- (.Z (Math|Vector|BreakVector (Transformation|GetActorLocation _array_element))) (.Z (Math|Vector|BreakVector (Transformation|GetWorldLocation (Variables|Debug|GetStaticMeshComponent))))) -1.5e+02)
      (Default|DamageHealth (.AsThird%20Person%20Character (Utilities|Casting|CastToThirdPersonCharacter _array_element)) 0.002 (.AsThird%20Person%20Character (Utilities|Casting|CastToThirdPersonCharacter _array_element))))))

(fn ConstructionScript)