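; BP_ManaPotion is a pickup that restores a portion of the ThirdPersonCharacter's Mana on overlap, capped at full.
; Overlap hides the bottle mesh and disables collision, then either adds mana or prints an already-full message.
; In both cases it spawns a heal-aura particle at the character's location, then destroys the emitter and itself after a short delay, so the potion is consumed even at full mana.
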(event EventBeginPlay)

(event Collision|EventActorBeginOverlap
  (params (OtherActor :type Actor%20Object%20Reference))
  (if (== (Utilities|GetClass OtherActor) "/Game/ThirdPersonBP/Blueprints/ThirdPersonCharacter.ThirdPersonCharacter_C")
    (Rendering|SetVisibility (Variables|Default|GetMBottle self) false false)
    (Collision|SetActorEnableCollision false)
    (bind _asthird_person_character (Utilities|Casting|CastToThirdPersonCharacter OtherActor))
    (if (< (Variables|/Game/ThirdPersonBP/Blueprints/ThirdPersonCharacter.ThirdPersonCharacter_C|GetMana _asthird_person_character) 1.0)
      (bind _output_get (Variables|/Game/ThirdPersonBP/Blueprints/ThirdPersonCharacter.ThirdPersonCharacter_C|SetMana _asthird_person_character (+ (Variables|/Game/ThirdPersonBP/Blueprints/ThirdPersonCharacter.ThirdPersonCharacter_C|GetMana _asthird_person_character) 0.2)))
      (if (>= _output_get 1.0)
        (Variables|/Game/ThirdPersonBP/Blueprints/ThirdPersonCharacter.ThirdPersonCharacter_C|SetMana _asthird_person_character 1.0))
      (else
        (Development|PrintString "Oh, You are already full mana.")))
    (bind _returnvalue (Effects|SpawnEmitteratLocation "/Game/FXVarietyPack/Particles/P_ky_healAura.P_ky_healAura" (Transformation|GetActorLocation _asthird_person_character) "0, 0, 0" "1.000000,1.000000,1.000000" false))
    (Utilities|FlowControl|Delay 3.0)
    (Components|DestroyComponent _returnvalue)
    (Actor|DestroyActor)))

(fn ConstructionScript)