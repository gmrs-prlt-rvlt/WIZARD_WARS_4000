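; BP_Spawner is an item spawner that keeps one random pickup from ItemsToSpawn at its own location and rotation.
; It attempts a spawn on BeginPlay and sets a looping respawn timer; the Respawn event retries after a delay.
; AttemptToSpawn spawns only when CurrentItem is invalid, otherwise printing a message and setting a one-shot timer.
; The random index's inclusive maximum is the array length, so it can fall out of range.
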(event EventBeginPlay
  (Utilities|Time|SetTimerbyEvent (delegate EventRespawn) 2.0 true)
  (CallFunction|AttempttoSpawn))

(event EventRespawn
  (Utilities|FlowControl|Delay 5.0)
  (CallFunction|AttempttoSpawn))

(fn ConstructionScript)

(fn AttempttoSpawn
  (Utilities|IsValid (Variables|Default|GetCurrentItem)
    (:Is%20Valid
      (Development|PrintString "Item already spawned")
      (Utilities|Time|SetTimerbyEvent (EventDispatchers|CreateEvent :!event AttempttoSpawn) 5.0))
    (:Is%20Not%20Valid
      (CallFunction|SpawnItem))))

(fn SpawnItem
  (bind _returnvalue (Game|SpawnActorfromClass (Utilities|Array|Get(acopy) (Variables|Default|GetItemsToSpawn) (Math|Random|RandomIntegerinRange 0 (Utilities|Array|Length (Variables|Default|GetItemsToSpawn)))) (Math|Transform|MakeTransform (Transformation|GetActorLocation) (Transformation|GetActorRotation)) "AdjustIfPossibleButAlwaysSpawn" self 0 0))
  (Variables|Default|SetCurrentItem _returnvalue))